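; BP_SB4K_HD_Perel is a space box actor, apparently the HD "Perel" variant, built from six face components.
; Its construction script sets the actor's 3D scale from the Scale variable and assigns a dedicated Mat_HD_Perel material to the first slot of the Up, Down, Left, Right, Front and Back faces.
; The file contains no runtime logic.
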(fn `UserConstructionScript`
  (`self.SetActorScale3D` (`self.Scale`))
  (`PrimitiveComponent.SetMaterial` (`self.Up`) 0 "/Game/SpaceBox_Dim/Materials/HD/Perel/Mat_HD_Perel_Up.Mat_HD_Perel_Up")
  (`PrimitiveComponent.SetMaterial` (`self.Right`) 0 "/Game/SpaceBox_Dim/Materials/HD/Perel/Mat_HD_Perel_Right.Mat_HD_Perel_Right")
  (`PrimitiveComponent.SetMaterial` (`self.Left`) 0 "/Game/SpaceBox_Dim/Materials/HD/Perel/Mat_HD_Perel_Left.Mat_HD_Perel_Left")
  (`PrimitiveComponent.SetMaterial` (`self.Front`) 0 "/Game/SpaceBox_Dim/Materials/HD/Perel/Mat_HD_Perel_Front.Mat_HD_Perel_Front")
  (`PrimitiveComponent.SetMaterial` (`self.Down`) 0 "/Game/SpaceBox_Dim/Materials/HD/Perel/Mat_HD_Perel_Down.Mat_HD_Perel_Down")
  (`PrimitiveComponent.SetMaterial` (`self.Back`) 0 "/Game/SpaceBox_Dim/Materials/HD/Perel/Mat_HD_Perel_Back.Mat_HD_Perel_Back"))
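; BP_SB4K_HD_Nidub is a space skybox actor that shows the HD Nidub variant from the SpaceBox content.
; Its construction script sets the actor's 3D scale from a Scale variable.
; It then assigns a matching Nidub material to the first slot of each of the six face components: Up, Down, Left, Right, Front and Back.
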(fn `UserConstructionScript`
  (`self.SetActorScale3D` (`self.Scale`))
  (`PrimitiveComponent.SetMaterial` (`self.Up`) 0 "/Game/SpaceBox_Dim/Materials/HD/Nidub/Mat_HD_Nidub_Up.Mat_HD_Nidub_Up")
  (`PrimitiveComponent.SetMaterial` (`self.Right`) 0 "/Game/SpaceBox_Dim/Materials/HD/Nidub/Mat_HD_Nidub_Right.Mat_HD_Nidub_Right")
  (`PrimitiveComponent.SetMaterial` (`self.Left`) 0 "/Game/SpaceBox_Dim/Materials/HD/Nidub/Mat_HD_Nidub_Left.Mat_HD_Nidub_Left")
  (`PrimitiveComponent.SetMaterial` (`self.Front`) 0 "/Game/SpaceBox_Dim/Materials/HD/Nidub/Mat_HD_Nidub_Front.Mat_HD_Nidub_Front")
  (`PrimitiveComponent.SetMaterial` (`self.Down`) 0 "/Game/SpaceBox_Dim/Materials/HD/Nidub/Mat_HD_Nidub_Down.Mat_HD_Nidub_Down")
  (`PrimitiveComponent.SetMaterial` (`self.Back`) 0 "/Game/SpaceBox_Dim/Materials/HD/Nidub/Mat_HD_Nidub_Back.Mat_HD_Nidub_Back"))
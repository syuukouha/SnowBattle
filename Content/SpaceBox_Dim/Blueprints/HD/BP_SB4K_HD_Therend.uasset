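; BP_SB4K_HD_Therend is a space box actor for the HD Therend variant, built from six face components.
; Its construction script sets the actor's scale from the Scale variable.
; It then assigns a matching Therend material to the first slot of the Up, Down, Left, Right, Front and Back faces.
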(fn `UserConstructionScript`
  (`self.SetActorScale3D` (`self.Scale`))
  (`PrimitiveComponent.SetMaterial` (`self.Up`) 0 "/Game/SpaceBox_Dim/Materials/HD/Therend/Mat_HD_Therend_Up.Mat_HD_Therend_Up")
  (`PrimitiveComponent.SetMaterial` (`self.Right`) 0 "/Game/SpaceBox_Dim/Materials/HD/Therend/Mat_HD_Therend_Right.Mat_HD_Therend_Right")
  (`PrimitiveComponent.SetMaterial` (`self.Left`) 0 "/Game/SpaceBox_Dim/Materials/HD/Therend/Mat_HD_Therend_Left.Mat_HD_Therend_Left")
  (`PrimitiveComponent.SetMaterial` (`self.Front`) 0 "/Game/SpaceBox_Dim/Materials/HD/Therend/Mat_HD_Therend_Front.Mat_HD_Therend_Front")
  (`PrimitiveComponent.SetMaterial` (`self.Down`) 0 "/Game/SpaceBox_Dim/Materials/HD/Therend/Mat_HD_Therend_Down.Mat_HD_Therend_Down")
  (`PrimitiveComponent.SetMaterial` (`self.Back`) 0 "/Game/SpaceBox_Dim/Materials/HD/Therend/Mat_HD_Therend_Back.Mat_HD_Therend_Back"))
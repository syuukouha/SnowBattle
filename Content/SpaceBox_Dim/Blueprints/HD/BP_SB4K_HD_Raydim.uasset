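; HD "Raydim" space box actor from the SpaceBox_Dim set, built from six face components: Up, Down, Left, Right, Front and Back.
; The construction script sets the actor's 3D scale from the Scale variable, then assigns each face its matching directional Raydim material on slot 0.
; It has no other graph logic, so all of the setup happens at construction.
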(fn `UserConstructionScript`
  (`self.SetActorScale3D` (`self.Scale`))
  (`PrimitiveComponent.SetMaterial` (`self.Up`) 0 "/Game/SpaceBox_Dim/Materials/HD/Raydim/Mat_HD_Raydim_Up.Mat_HD_Raydim_Up")
  (`PrimitiveComponent.SetMaterial` (`self.Right`) 0 "/Game/SpaceBox_Dim/Materials/HD/Raydim/Mat_HD_Raydim_Right.Mat_HD_Raydim_Right")
  (`PrimitiveComponent.SetMaterial` (`self.Left`) 0 "/Game/SpaceBox_Dim/Materials/HD/Raydim/Mat_HD_Raydim_Left.Mat_HD_Raydim_Left")
  (`PrimitiveComponent.SetMaterial` (`self.Front`) 0 "/Game/SpaceBox_Dim/Materials/HD/Raydim/Mat_HD_Raydim_Front.Mat_HD_Raydim_Front")
  (`PrimitiveComponent.SetMaterial` (`self.Down`) 0 "/Game/SpaceBox_Dim/Materials/HD/Raydim/Mat_HD_Raydim_Down.Mat_HD_Raydim_Down")
  (`PrimitiveComponent.SetMaterial` (`self.Back`) 0 "/Game/SpaceBox_Dim/Materials/HD/Raydim/Mat_HD_Raydim_Back.Mat_HD_Raydim_Back"))
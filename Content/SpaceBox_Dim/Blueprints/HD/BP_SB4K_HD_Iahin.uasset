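; BP_SB4K_HD_Iahin is an actor that forms the HD Iahin variant of a space box, judging by its naming.
; Its construction script sets the actor's 3D scale from the Scale variable.
; It then assigns a dedicated Iahin material to slot 0 of each of the six face components: Up, Down, Left, Right, Front and Back.
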(fn `UserConstructionScript`
  (`self.SetActorScale3D` (`self.Scale`))
  (`PrimitiveComponent.SetMaterial` (`self.Up`) 0 "/Game/SpaceBox_Dim/Materials/HD/Iahin/Mat_HD_Iahin_Up.Mat_HD_Iahin_Up")
  (`PrimitiveComponent.SetMaterial` (`self.Right`) 0 "/Game/SpaceBox_Dim/Materials/HD/Iahin/Mat_HD_Iahin_Right.Mat_HD_Iahin_Right")
  (`PrimitiveComponent.SetMaterial` (`self.Left`) 0 "/Game/SpaceBox_Dim/Materials/HD/Iahin/Mat_HD_Iahin_Left.Mat_HD_Iahin_Left")
  (`PrimitiveComponent.SetMaterial` (`self.Front`) 0 "/Game/SpaceBox_Dim/Materials/HD/Iahin/Mat_HD_Iahin_Front.Mat_HD_Iahin_Front")
  (`PrimitiveComponent.SetMaterial` (`self.Down`) 0 "/Game/SpaceBox_Dim/Materials/HD/Iahin/Mat_HD_Iahin_Down.Mat_HD_Iahin_Down")
  (`PrimitiveComponent.SetMaterial` (`self.Back`) 0 "/Game/SpaceBox_Dim/Materials/HD/Iahin/Mat_HD_Iahin_Back.Mat_HD_Iahin_Back"))
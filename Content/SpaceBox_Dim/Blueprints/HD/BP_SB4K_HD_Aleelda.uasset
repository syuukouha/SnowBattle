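; BP_SB4K_HD_Aleelda is a space skybox actor for the HD Aleelda backdrop in the SpaceBox set.
; Its construction script sets the actor's scale from a Scale variable, then assigns a dedicated Aleelda material to each of six face components: Up, Down, Left, Right, Front and Back.
; The script contains only this setup, with no runtime logic.
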(fn `UserConstructionScript`
  (`self.SetActorScale3D` (`self.Scale`))
  (`PrimitiveComponent.SetMaterial` (`self.Up`) 0 "/Game/SpaceBox_Dim/Materials/HD/Aleelda/Mat_HD_Aleelda_Up.Mat_HD_Aleelda_Up")
  (`PrimitiveComponent.SetMaterial` (`self.Right`) 0 "/Game/SpaceBox_Dim/Materials/HD/Aleelda/Mat_HD_Aleelda_Right.Mat_HD_Aleelda_Right")
  (`PrimitiveComponent.SetMaterial` (`self.Left`) 0 "/Game/SpaceBox_Dim/Materials/HD/Aleelda/Mat_HD_Aleelda_Left.Mat_HD_Aleelda_Left")
  (`PrimitiveComponent.SetMaterial` (`self.Front`) 0 "/Game/SpaceBox_Dim/Materials/HD/Aleelda/Mat_HD_Aleelda_Front.Mat_HD_Aleelda_Front")
  (`PrimitiveComponent.SetMaterial` (`self.Down`) 0 "/Game/SpaceBox_Dim/Materials/HD/Aleelda/Mat_HD_Aleelda_Down.Mat_HD_Aleelda_Down")
  (`PrimitiveComponent.SetMaterial` (`self.Back`) 0 "/Game/SpaceBox_Dim/Materials/HD/Aleelda/Mat_HD_Aleelda_Back.Mat_HD_Aleelda_Back"))
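; BP_SB4K_HD_Losyn is a skybox actor in the SpaceBox set that displays the HD Losyn environment on six faces.
; Its construction script scales the actor by the Scale variable, then assigns a dedicated Losyn material to each of the Up, Down, Left, Right, Front and Back components.
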(fn `UserConstructionScript`
  (`self.SetActorScale3D` (`self.Scale`))
  (`PrimitiveComponent.SetMaterial` (`self.Up`) 0 "/Game/SpaceBox_Dim/Materials/HD/Losyn/Mat_HD_Losyn_Up.Mat_HD_Losyn_Up")
  (`PrimitiveComponent.SetMaterial` (`self.Right`) 0 "/Game/SpaceBox_Dim/Materials/HD/Losyn/Mat_HD_Losyn_Right.Mat_HD_Losyn_Right")
  (`PrimitiveComponent.SetMaterial` (`self.Left`) 0 "/Game/SpaceBox_Dim/Materials/HD/Losyn/Mat_HD_Losyn_Left.Mat_HD_Losyn_Left")
  (`PrimitiveComponent.SetMaterial` (`self.Front`) 0 "/Game/SpaceBox_Dim/Materials/HD/Losyn/Mat_HD_Losyn_Front.Mat_HD_Losyn_Front")
  (`PrimitiveComponent.SetMaterial` (`self.Down`) 0 "/Game/SpaceBox_Dim/Materials/HD/Losyn/Mat_HD_Losyn_Down.Mat_HD_Losyn_Down")
  (`PrimitiveComponent.SetMaterial` (`self.Back`) 0 "/Game/SpaceBox_Dim/Materials/HD/Losyn/Mat_HD_Losyn_Back.Mat_HD_Losyn_Back"))